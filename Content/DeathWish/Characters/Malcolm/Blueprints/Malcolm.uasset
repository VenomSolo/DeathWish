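; Malcolm character Blueprint that tracks the mouse cursor to compute a rotation for a corpse.
; BeginPlay shows the first player's mouse cursor.
; Each tick traces under the cursor on the Camera channel and stores CorpseRotation, with pitch fixed at a right angle, the actor's roll, and yaw summing the look-at yaw toward the impact point and the actor's own yaw.
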(event EventBeginPlay
  (Variables|/Script/Engine.PlayerController|SetbShowMouseCursor (Game|GetPlayerController 0) true))

(event Collision|EventActorBeginOverlap
  (params (OtherActor :type Actor%20Object%20Reference)))

(event EventTick
  (params (DeltaSeconds :type Float%20%28single-precision%29))
  (bind _returnvalue (Transformation|GetActorRotation))
  (bind (_roll _pitch _yaw) (Math|Rotator|BreakRotator _returnvalue))
  (Variables|Default|SetCorpseRotation (Math|Rotator|MakeRotator _roll 9e+01 (+ (.Yaw (Math|Rotator|BreakRotator (Math|Rotator|FindLookatRotation (Transformation|GetActorLocation) (.ImpactPoint (Collision|BreakHitResult (.HitResult (Game|Player|GetHitResultUnderCursorbyChannel (Game|GetPlayerController 0) "TraceTypeQuery2" true))))))) _yaw))))

(fn ConstructionScript)